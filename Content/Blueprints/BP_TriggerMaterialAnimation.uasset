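; BP_TriggerMaterialAnimation plays a disintegration material animation when Space Bar is pressed.
; While animating, Tick advances an interpolation value by speed and delta time, samples a float curve with it, and writes the result to a named scalar in a Material Parameter Collection.
; Animation stops once the value exceeds one, and the value is never reset.
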(event `self.ReceiveTick`
  (params (DeltaSeconds :type "Float (single-precision)"))
  (if (`self.IsAnimating`)
    (bind _output_get (set `self.InterpolationValue` (+ (`self.InterpolationValue`) (* (`self.AnimationSpeed`) DeltaSeconds))))
    (`KismetMaterialLibrary.SetScalarParameterValue` (`self.DesintegrationParameterCollection`) (`self.Parameter Name`) (`CurveFloat.GetFloatValue` (`self.DesintegrationCurve`) _output_get))
    (if (> (`self.InterpolationValue`) 1.0)
      (set `self.IsAnimating` false))))

(event `Key|SpaceBar`
  (params (Key :type "Key Structure"))
  (:`Pressed`
    (set `self.IsAnimating` true)))

(fn `UserConstructionScript`)